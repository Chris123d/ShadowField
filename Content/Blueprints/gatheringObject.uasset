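; Gatherable object actor that highlights and becomes active while another actor overlaps it.
; Overlap begin and end toggle the Active flag and switch the mesh's custom depth stencil value, with debug prints.
; The construction script creates a dynamic instance of PP_OutlineColored on the mesh's first material slot and stores it.
; Gather is a stub that only prints a message and is not called within this Blueprint.
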(event `self.ReceiveActorBeginOverlap`
  (params (OtherActor :type "Actor Object Reference"))
  (`self.setActive`))

(event `self.ReceiveActorEndOverlap`
  (params (OtherActor :type "Actor Object Reference"))
  (`self.setInactive`))

(fn `gather`
  (`KismetSystemLibrary.PrintString` "Gathering"))

(fn `setActive`
  (`KismetSystemLibrary.PrintString` "Activating")
  (`PrimitiveComponent.SetCustomDepthStencilValue` (`self.Mesh`) 254)
  (set `self.Active` true))

(fn `setInactive`
  (`KismetSystemLibrary.PrintString` "Deactivating")
  (`PrimitiveComponent.SetCustomDepthStencilValue` (`self.Mesh`) 0)
  (set `self.Active` false))

(fn `UserConstructionScript`
  (bind _returnvalue (`PrimitiveComponent.CreateDynamicMaterialInstance` (`self.Mesh`) 0 "/Game/Blueprints/PP_OutlineColored.PP_OutlineColored"))
  (set `self.Material` _returnvalue))