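; Flashlight pickup actor that fills the player character's flashlight inventory slot.
; Pickup is enabled two seconds after BeginPlay.
; When its box is overlapped, it checks the player ThirdPersonCharacter's FlashlightSlotItem, then either sets it and destroys itself or prints that only one flashlight is allowed.
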(event `self.ReceiveBeginPlay`
  (`KismetSystemLibrary.Delay` 2.0)
  (set `self.canPickup` true))

(event `self.Box.OnComponentBeginOverlap`
  (params (OverlappedComponent :type "PrimitiveComponent Object Reference") (OtherActor :type "Actor Object Reference") (OtherComp :type "PrimitiveComponent Object Reference") (OtherBodyIndex :type Integer) (bFromSweep :type Boolean) (SweepResult :type "HitResult Structure (by ref)"))
  (if (`self.canPickup`)
    (bind _asthird_person_character (cast `/Game/ThirdPersonBP/Blueprints/ThirdPersonCharacter` (`GameplayStatics.GetPlayerCharacter` 0)))
    (if (== (`/Game/ThirdPersonBP/Blueprints/ThirdPersonCharacter.flashlight-Slot-Item` _asthird_person_character) 0)
      (set `/Game/ThirdPersonBP/Blueprints/ThirdPersonCharacter.flashlight-Slot-Item` 1 _asthird_person_character)
      (`self.K2_DestroyActor`)
      (else
        (`KismetSystemLibrary.PrintString` "Can only have one flashlight.")))))

(fn `UserConstructionScript`)